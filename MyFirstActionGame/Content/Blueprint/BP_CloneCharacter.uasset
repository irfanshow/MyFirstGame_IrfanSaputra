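; Player-controllable clone character that carries an E-11 blaster and handles basic movement, look and jump input.
; On BeginPlay it spawns BP_Blaster_E11 at the mesh's right-side blaster socket and snaps it to that socket.
; Look axes feed controller yaw and pitch, while movement axes push along the capsule's forward and right vectors.
; It contains no firing logic, and jump responds only to the press.
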(event EventBeginPlay
  (bind _returnvalue (Game|SpawnActorfromClass "/Game/Blueprint/BP_Blaster_E11.BP_Blaster_E11_C" (Transformation|GetSocketTransform (Variables|Character|GetMesh) "Socker_R_Blaster" "RTS_World") "Undefined" "MultiplyWithRoot" 0 0))
  (Transformation|AttachComponentToComponent _returnvalue (Variables|Character|GetMesh) "Socker_R_Blaster" "SnapToTarget" "SnapToTarget" "SnapToTarget" true))

(event Input|ActionEvents|InputActionJump
  (params (Key :type Key%20Structure :default "None"))
  ;[1 1 1] Player Jump
  (:Pressed
    (Character|Jump)))

(event Input|AxisEvents|InputAxisTurn
  (params (AxisValue :type Float%20%28single-precision%29))
  ;[1 1 1] Look Up and Turn
  (Pawn|Input|AddControllerYawInput AxisValue))

(event Input|AxisEvents|InputAxisLookUp
  (params (AxisValue :type Float%20%28single-precision%29))
  ;[1 1 1] Look Up and Turn
  (Pawn|Input|AddControllerPitchInput AxisValue))

(event Input|AxisEvents|InputAxisForwardBackwardMove
  (params (AxisValue :type Float%20%28single-precision%29))
  ;[1 1 1] Player Movement
  (Pawn|Input|AddMovementInput (Math|Vector|GetForwardVector (Variables|Collision|GetCapsuleComponent)) AxisValue false))

(event Input|AxisEvents|InputAxisLeftRightMove
  (params (AxisValue :type Float%20%28single-precision%29))
  ;[1 1 1] Player Movement
  (Pawn|Input|AddMovementInput (Math|Vector|GetRightVector (Variables|Collision|GetCapsuleComponent)) AxisValue false))

(fn ConstructionScript)