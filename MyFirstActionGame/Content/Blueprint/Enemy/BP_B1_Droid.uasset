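; B1 battle droid enemy that wanders randomly, chases and shoots the player on sight, and awards score when killed.
; PawnSensing fires lasers and sets a seen flag that a retriggerable delay clears when sightings stop.
; Tick uses that flag to choose chase or patrol AIMoveTo, updates a camera-facing health bar, and handles death at zero health.
; Weapon-spawn, input-mapping and muzzle-fire functions exist but are not called here.
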(event OnSeePawn(PawnSensing)
  (params (Pawn :type Pawn%20Object%20Reference))
  ;[1 1 1] AI Folllow Player And Shoot
  (bind _asbp_clone_character (Utilities|Casting|CastToBP_CloneCharacter Pawn))
  (Variables|Default|SetPlayer%20Followed _asbp_clone_character)
  (Utilities|FlowControl|Sequence
    (:then_0
      (Variables|Default|SetisSeePlayer? true)
      (Game|SpawnActorfromClass "/Game/Blueprint/BP_RedLaser_Bullet.BP_RedLaser_Bullet_C" (Transformation|GetWorldTransform (Variables|Default|GetProjectileSpawn)) "Undefined" "MultiplyWithRoot" 0 0)
      (Audio|PlaySoundatLocation "/Game/Assets/Sound_Assets/E-5_SFX/SC_E5_SFX.SC_E5_SFX" (Transformation|GetWorldLocation (Variables|Character|GetMesh)) "0, 0, 0" 1.0 1.0 0.0 0 0 0 0))
    (:then_1
      (Utilities|FlowControl|RetriggerableDelay 0.6)
      (Variables|Default|SetisSeePlayer? false))))

(event Custom|Move%20NPC
  ;[1 1 1] AI Patrol
  (AI|AIMoveTo self (.RandomLocation (AI|Navigation|GetRandomReachablePointinRadius (Transformation|GetActorLocation) 1e+03 0 0)) 0 5.0 false))

(event Game|Damage|EventAnyDamage
  (params (Damage :type Float%20%28single-precision%29) (DamageType :type Damage%20Type%20Object%20Reference) (InstigatedBy :type Controller%20Object%20Reference) (DamageCauser :type Actor%20Object%20Reference))
  ;[1 1 1] Take Damage
  (if (not (<= (Variables|Default|GetcurrentHealth) 0.0))
    (bind _output_get (Variables|Default|SetcurrentHealth (- (Variables|Default|GetcurrentHealth) Damage)))
    (Development|PrintString (Utilities|String|Append "Enemy : " (Utilities|String|ToString(Float) _output_get)))))

(event EventTick
  (params (DeltaSeconds :type Float%20%28single-precision%29))
  (bind _healthbar_widget (Variables|Default|GetHealthBar%20Widget))
  ;[1 1 1] Evenet Tick
  (bind _aswbp_health_bar (Utilities|Casting|CastToWBP_HealthBar (UserInterface|GetWidget (Variables|Default|GetHealthBar%20Widget))))
  (bind _output_get (Variables|Default|SetWBP%20Health%20Bar _aswbp_health_bar))
  (Default|SetHealth _output_get (Variables|Default|GetcurrentHealth) (Variables|Default|GetmaxHealth))
  (Transformation|SetWorldRotation _healthbar_widget (Math|Rotator|FindLookatRotation (Transformation|GetWorldLocation _healthbar_widget) (Transformation|GetWorldLocation (Variables|/Script/Engine.PlayerCameraManager|GetTransformComponent (Game|GetPlayerCameraManager 0)))) false false)
  (if (<= (Variables|Default|GetcurrentHealth) 0.0)
    (Utilities|FlowControl|DoOnce false
      (:Completed
        (if (<= (Variables|Default|GetcurrentHealth) 0.0)
          (CallFunction|OnEnemyDeath)
          (Utilities|FlowControl|Delay 2.0)
          (Actor|DestroyActor))))
    (elif (Variables|Default|GetisSeePlayer?)
      (Utilities|FlowControl|DoOnce false :!label _label
        (:Completed
          (AI|AIMoveTo self (Transformation|GetActorLocation (Variables|Default|GetPlayer%20Followed)) 0 5.0 false
            (:OnSuccess
              (goto _label Reset)))))
      (else
        (Utilities|FlowControl|DoOnce false :!label _label_2
          (:Completed
            (CallFunction|MoveNPC)
            (Utilities|FlowControl|Delay 3.0)
            (goto _label_2 Reset)))))))

(event EventBeginPlay
  ;[1 1 1] BeginPlay
  (bind _asbp_clone_character (Utilities|Casting|CastToBP_CloneCharacter (Game|GetPlayerCharacter 0)))
  (Variables|Default|SetBP%20Clone%20Character _asbp_clone_character))

(fn ConstructionScript)

(fn SpawnRifle
  (bind _returnvalue (Game|SpawnActorfromClass "/Game/Blueprint/Weapon/BP_Blaster_E11.BP_Blaster_E11_C" (Transformation|GetSocketTransform (Variables|Character|GetMesh) "Holster_Weapon_Main" "RTS_World") "Undefined" "MultiplyWithRoot" 0 "/Game/Blueprint/Weapon/DA_Blaster_E11.DA_Blaster_E11" 0))
  (Variables|Default|SetWeapon (Variables|/Game/Blueprint/Weapon/BP_Blaster_E11.BP_Blaster_E11_C|GetWeaponData _returnvalue))
  (Transformation|AttachComponentToComponent _returnvalue (Variables|Character|GetMesh) "Holster_Weapon_Main" "SnapToTarget" "SnapToTarget" "SnapToTarget" true)
  (Actor|DestroyActor _returnvalue)
  (Components|StaticMesh|SetStaticMesh (Variables|Default|GetHolsterWeaponMesh) (Variables|/Game/Blueprint/Weapon/BP_Weapon_Data.BP_Weapon_Data_C|GetMesh (Variables|Default|GetWeapon))))

(fn SetController
  (bind _asplayer_controller (Utilities|Casting|CastToPlayerController (Pawn|GetController)))
  (Input|AddMappingContext (PlayerController|LocalPlayerSubsystems|GetEnhancedInputLocalPlayerSubsystem _asplayer_controller) "/Game/Blueprint/Input/IMC_CloneTrooper.IMC_CloneTrooper" 0 "(bIgnoreAllPressedKeysUntilRelease=True,bForceImmediately=False,bNotifyUserSettings=False)"))

(fn CheckWeaponandHolster
  (return (and (Utilities|IsValid (Variables|Default|GetWeapon)) (not false))))

(fn FireLaser
  (Game|SpawnActorfromClass "/Game/Blueprint/BP_RedLaser_Bullet.BP_RedLaser_Bullet_C" (Transformation|GetSocketTransform (Variables|Default|GetWeaponMesh) "Muzzle_Socket" "RTS_World") "Undefined" "MultiplyWithRoot" 0 0))

(fn OnEnemyDeath
  (Variables|/Game/Blueprint/BP_CloneCharacter.BP_CloneCharacter_C|SetPlayerScore (Variables|Default|GetBP%20Clone%20Character) (+ (Variables|Default|GetScore) 10))
  (Variables|/Script/AIModule.PawnSensingComponent|SetbSeePawns (Variables|Default|GetPawnSensing) false)
  (Pawn|Components|CharacterMovement|DisableMovement (Variables|Character|GetCharacterMovement))
  (Audio|PlaySoundatLocation "/Game/Assets/Sound_Assets/Droid_Death/SC_Droid_Death_SFX.SC_Droid_Death_SFX" (Transformation|GetWorldLocation (Variables|Character|GetMesh)) "0, 0, 0" 1.0 1.0 0.0 0 0 0 0)
  (Animation|PlayAnimMontage "/Game/Assets/Animations_Assets/B1_Droid_Animation/AM_B1_Death_2_Montage.AM_B1_Death_2_Montage" 1.0 "None")
  (Rendering|SetVisibility (Variables|Default|GetHealthBar%20Widget) false false))